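; Character Blueprint with a custom event that sets IsOnScreen by projecting the actor's location to screen and comparing it against the viewport bounds.
; An unconnected visibility prototype sweeps debug line traces from the screen's vertical centerline across the player pawn's extents, using oscillating lerp alphas.
; That disconnected loop prints whether a hit pawn is within the viewport, but never runs, as BeginPlay is empty.
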(event `Check Is On Screen`
  (bind (_returnvalue_x _returnvalue_y) (`KismetMathLibrary.BreakVector2D` (`WidgetLayoutLibrary.GetViewportSize`)))
  (bind _screenlocation (`PlayerController.ProjectWorldLocationToScreen` (`GameplayStatics.GetPlayerController` 0) (`self.K2_GetActorLocation`) false))
  (set `self.Is On Screen?` (and (> (`KismetMathLibrary.BreakVector2D` _screenlocation) 0.0) (> (`.Y` (`KismetMathLibrary.BreakVector2D` _screenlocation)) 0.0) (< (`KismetMathLibrary.BreakVector2D` _screenlocation) _returnvalue_x) (< (`.Y` (`KismetMathLibrary.BreakVector2D` _screenlocation)) _returnvalue_y))))

(event `self.ReceiveBeginPlay`)

(fn `UserConstructionScript`)