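; BackoutOfEpisode is a one-shot trigger actor that relocates the player, apparently to exit an episode.
; The first overlap with its Box, unfiltered by actor, moves the player pawn to the NewPosition actor's location and sets the controller's rotation to match.
; It then sets the pawn's spotlight intensity and deactivates its own root component, with DoOnce preventing repeats.
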(event `self.Box.OnComponentBeginOverlap`
  (params (OverlappedComponent :type "PrimitiveComponent Object Reference") (OtherActor :type "Actor Object Reference") (OtherComp :type "PrimitiveComponent Object Reference") (OtherBodyIndex :type Integer) (bFromSweep :type Boolean) (SweepResult :type "HitResult Structure (by ref)"))
  (bind _returnvalue (`GameplayStatics.GetPlayerPawn` 0))
  (bind _newposition (`self.NewPosition`))
  (`/Engine/EditorBlueprintResources/StandardMacros.DoOnce` false
    (:`Completed`
      (`self.K2_SetActorLocation` _returnvalue (`self.K2_GetActorLocation` _newposition) false false)
      (`Controller.SetControlRotation` (`GameplayStatics.GetPlayerController` 0) (`self.K2_GetActorRotation` _newposition))
      (`LightComponent.SetIntensity` (`self.GetComponentByClass` _returnvalue "/Script/Engine.SpotLightComponent") 2400.0)
      (`ActorComponent.SetActive` (`self.DefaultSceneRoot`) false false))))

(fn `UserConstructionScript`)