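; LockedCupboard is a cupboard that the player can open by interacting with it once its key has been picked up.
; Trigger overlap events open and close a gate on Tick, which polls the Player pawn's Interact flag and the Key's HasPlayerPickedUp flag while open.
; When both are set, a DoOnce plays the door's opening animation without looping and turns off the Box's collision.
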(event `self.ReceiveTick`
  (params (DeltaSeconds :type "Float (single-precision)"))
  (`/Engine/EditorBlueprintResources/StandardMacros.Gate` true :!label _label
    (:`Exit`
      (bind _asplayer (cast `/Game/Blueprints/Player` (`GameplayStatics.GetPlayerPawn` 0)))
      (if (`/Game/Blueprints/Player.Interact` _asplayer)
        (if (`/Game/Blueprints/Key.HasPlayerPickedUp` (`self.Key`))
          (`/Engine/EditorBlueprintResources/StandardMacros.DoOnce` false
            (:`Completed`
              (`SkeletalMeshComponent.PlayAnimation` (`self.Door`) "/Game/Models/Cupboard_Door_Anim_Open.Cupboard_Door_Anim_Open" false)
              (`PrimitiveComponent.SetCollisionEnabled` (`self.Box`) "NoCollision"))))))))

(event `self.Trigger.OnComponentBeginOverlap`
  (params (OverlappedComponent :type "PrimitiveComponent Object Reference") (OtherActor :type "Actor Object Reference") (OtherComp :type "PrimitiveComponent Object Reference") (OtherBodyIndex :type Integer) (bFromSweep :type Boolean) (SweepResult :type "HitResult Structure (by ref)"))
  (goto _label :!via `Open`))

(event `self.Trigger.OnComponentEndOverlap`
  (params (OverlappedComponent :type "PrimitiveComponent Object Reference") (OtherActor :type "Actor Object Reference") (OtherComp :type "PrimitiveComponent Object Reference") (OtherBodyIndex :type Integer))
  (goto _label :!via `Close`))

(fn `UserConstructionScript`)