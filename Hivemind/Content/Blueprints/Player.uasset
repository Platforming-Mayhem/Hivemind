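; Player character Blueprint that handles movement, look input and an Interact flag, plus a debug check of whether the IDK actor is visible.
; A repeating BeginPlay loop sweeps line traces from screen points across that actor's bounds, but ignores the hits and prints visibility from its projected screen position alone.
; Tick applies movement unless FreezePosition is set; look input and the BodyAnimations Move flag update only while FreezeRotation is true.
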(event `self.ReceiveBeginPlay`
  (bind _returnvalue (`self.GetActorUpVector`))
  (bind (_returnvalue_x _returnvalue_y) (`KismetMathLibrary.BreakVector2D` (`WidgetLayoutLibrary.GetViewportSize`)))
  (bind _returnvalue_2 (`GameplayStatics.GetPlayerController` 0))
  (bind (_returnvalue_x_2 _returnvalue_y_2) (`KismetMathLibrary.BreakVector2D` (`WidgetLayoutLibrary.GetViewportSize`)))
  (bind _idk (`self.IDK`))
  (bind _returnvalue_3 (`self.GetActorRightVector` (`GameplayStatics.GetPlayerCharacter` 0)))
  (bind _returnvalue_4 (/ _returnvalue_x 2.0))
  (bind _returnvalue_5 (`self.K2_GetActorLocation` _idk))
  (bind (_origin _boxextent) (`self.GetActorBounds` _idk false false))
  (bind _screenlocation (`PlayerController.ProjectWorldLocationToScreen` (`GameplayStatics.GetPlayerController` 0) _returnvalue_5 false))
  (while (< (`self.Lerp float`) 0.0) :!label _label
    (bind _output_get (set `self.Lerp float` (+ (stale _output_get) 0.1)))
    (bind _outhit (`KismetSystemLibrary.LineTraceSingle` (`KismetMathLibrary.VLerp` (`PlayerController.DeprojectScreenPositionToWorld` _returnvalue_2 _returnvalue_4 0.0) (`PlayerController.DeprojectScreenPositionToWorld` _returnvalue_2 _returnvalue_4 _returnvalue_y) (`self.Lerp float`)) (`KismetMathLibrary.MakeVector` (.x (`KismetMathLibrary.VLerp` (+ (* _returnvalue_3 (.z _boxextent)) _returnvalue_5) (+ (* _returnvalue_3 (* (.z _boxextent) -1.0)) _returnvalue_5) (`self.Lerp float XY`))) (.y (`KismetMathLibrary.VLerp` (+ (* _returnvalue_3 (.z _boxextent)) _returnvalue_5) (+ (* _returnvalue_3 (* (.z _boxextent) -1.0)) _returnvalue_5) (`self.Lerp float XY`))) (.z (`KismetMathLibrary.VLerp` (+ (* _returnvalue (.z _boxextent)) _returnvalue_5) (+ (* _returnvalue (* (.z _boxextent) -1.0)) _returnvalue_5) (`self.Lerp float`)))) "TraceTypeQuery1" :!label _label_2))
    (if true
      (if (and (> (`KismetMathLibrary.BreakVector2D` _screenlocation) 0.0) (> (`.Y` (`KismetMathLibrary.BreakVector2D` _screenlocation)) 0.0) (< (`KismetMathLibrary.BreakVector2D` _screenlocation) _returnvalue_x_2) (< (`.Y` (`KismetMathLibrary.BreakVector2D` _screenlocation)) _returnvalue_y_2))
        (`KismetSystemLibrary.PrintString` "can see")
        (else
          (`KismetSystemLibrary.PrintString` "Can not see")))))
  (bind _output_get_2 (set `self.Lerp float XY` (+ (stale _output_get_2) (`self.Direction`))))
  (if (<= _output_get_2 0.0)
    (set `self.Direction` 0.1)
    (elif (> _output_get_2 0.0)
      (set `self.Direction` -1.0)))
  (while (> (`self.Lerp float`) 0.0)
    (bind _output_get_3 (set `self.Lerp float` (- (stale _output_get_3) 0.1)))
    (goto _label_2))
  (`KismetSystemLibrary.Delay` 0.1)
  (goto _label))

(event `InputAction|Interact`
  (params (Key :type "Key Structure"))
  (:`Pressed`
    (set `self.Interact` true))
  (:`Released`
    (set `self.Interact` false)))

(event `self.ReceiveTick`
  (params (DeltaSeconds :type "Float (single-precision)"))
  (bind _mesh (`self.Mesh`))
  (if (not (`self.FreezePosition`))
    (`self.AddMovementInput` (`SceneComponent.GetRightVector` _mesh) (* (`self.GetInputAxisValue`) (`self.Speed`)))
    (`self.AddMovementInput` (`SceneComponent.GetForwardVector` _mesh) (* (* (`self.GetInputAxisValue`) -1.0) (`self.Speed`))))
  (if (`self.FreezeRotation`)
    (`self.AddControllerYawInput` (`self.GetInputAxisKeyValue`))
    (`self.AddControllerPitchInput` (* (`self.GetInputAxisKeyValue`) -1.0))
    (bind _returnvalue (`PrimitiveComponent.GetPhysicsLinearVelocity` (`self.CapsuleComponent`) "None"))
    (bind _asbody_animations (cast `/Game/Animations/BodyAnimations` (`SkeletalMeshComponent.GetAnimInstance` (`self.Mesh`))))
    (if (> (`KismetMathLibrary.VSize` _returnvalue) 0.0)
      (set `/Game/Animations/BodyAnimations.move` true _asbody_animations)
      (else
        (set `/Game/Animations/BodyAnimations.move` false _asbody_animations)))))

(fn `UserConstructionScript`)