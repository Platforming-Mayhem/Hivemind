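; Keycard-locked door Blueprint that opens and closes as actors enter and leave its trigger, once the keycard has been picked up.
; Trigger overlaps check the Keycard's pickup flag, then play the opening or closing animation and toggle the blocking Box's collision off or on.
; BeginPlay reuses the closing branch without the keycard check, so the door plays its closing animation and starts with collision enabled.
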(event `self.Trigger.OnComponentBeginOverlap`
  (params (OverlappedComponent :type "PrimitiveComponent Object Reference") (OtherActor :type "Actor Object Reference") (OtherComp :type "PrimitiveComponent Object Reference") (OtherBodyIndex :type Integer) (bFromSweep :type Boolean) (SweepResult :type "HitResult Structure (by ref)"))
  (if (`/Game/Blueprints/Keycard.hasPlayerPickedUp` (`self.Keycard`))
    (`SkeletalMeshComponent.PlayAnimation` (`self.Door`) "/Game/Models/Door_Anim_Armature_Opening.Door_Anim_Armature_Opening" false)
    (`PrimitiveComponent.SetCollisionEnabled` (`self.Box`) "NoCollision")))

(event `self.Trigger.OnComponentEndOverlap`
  (params (OverlappedComponent :type "PrimitiveComponent Object Reference") (OtherActor :type "Actor Object Reference") (OtherComp :type "PrimitiveComponent Object Reference") (OtherBodyIndex :type Integer))
  (if (`/Game/Blueprints/Keycard.hasPlayerPickedUp` (`self.Keycard`))
    (`SkeletalMeshComponent.PlayAnimation` (`self.Door`) "/Game/Models/Door_Anim_Armature_Closing.Door_Anim_Armature_Closing" false :!label _label)
    (`PrimitiveComponent.SetCollisionEnabled` (`self.Box`) "QueryAndPhysics")))

(event `self.ReceiveBeginPlay`
  (goto _label))

(fn `UserConstructionScript`)