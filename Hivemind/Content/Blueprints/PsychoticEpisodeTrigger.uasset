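; PsychoticEpisodeTrigger is a one-shot trigger volume that relocates the player, named for a psychotic episode.
; The first overlap of its Box by any actor passes a DoOnce, casts player pawn 0 to Player and deactivates DefaultSceneRoot.
; It then moves the player to the Loc actor's location without sweeping and matches the controller's rotation to Loc.
; A disconnected node chain for zeroing the player's spotlight intensity never runs.
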(event `self.Box.OnComponentBeginOverlap`
  (params (OverlappedComponent :type "PrimitiveComponent Object Reference") (OtherActor :type "Actor Object Reference") (OtherComp :type "PrimitiveComponent Object Reference") (OtherBodyIndex :type Integer) (bFromSweep :type Boolean) (SweepResult :type "HitResult Structure (by ref)"))
  (bind _loc (`self.Loc`))
  (`/Engine/EditorBlueprintResources/StandardMacros.DoOnce` false
    (:`Completed`
      (bind _asplayer (cast `/Game/Blueprints/Player` (`GameplayStatics.GetPlayerPawn` 0)))
      (`ActorComponent.SetActive` (`self.DefaultSceneRoot`) false false)
      (`self.K2_SetActorLocation` _asplayer (`self.K2_GetActorLocation` _loc) false false)
      (`Controller.SetControlRotation` (`GameplayStatics.GetPlayerController` 0) (`self.K2_GetActorRotation` _loc)))))

(fn `UserConstructionScript`)