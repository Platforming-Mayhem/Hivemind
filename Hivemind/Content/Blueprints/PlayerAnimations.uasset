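; Player character Blueprint that drives movement and camera look; despite its name, it contains no animation logic.
; Every Tick it polls the WS and DA input axes, scales them by Speed and feeds them to AddMovementInput.
; WS moves along the mesh's right vector and DA along its negated forward vector.
; Two axis key values feed controller yaw and negated pitch.
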(event `self.ReceiveTick`
  (params (DeltaSeconds :type "Float (single-precision)"))
  (`self.AddMovementInput` (`SceneComponent.GetRightVector` (`self.Mesh`)) (* (`self.GetInputAxisValue`) (`self.speed`)))
  (`self.AddMovementInput` (`SceneComponent.GetForwardVector` (`self.Mesh`)) (* (`self.GetInputAxisValue`) (`self.speed`) -1.0))
  (`self.AddControllerYawInput` (`self.GetInputAxisKeyValue`))
  (`self.AddControllerPitchInput` (* (`self.GetInputAxisKeyValue`) -1.0)))

(fn `UserConstructionScript`)